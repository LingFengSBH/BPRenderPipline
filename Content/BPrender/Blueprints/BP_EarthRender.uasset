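; Blueprint software rasterizer that renders two meshes into deferred-style render targets and a spotlight shadow map.
; BeginPlay publishes the spotlight's basis to MPC_RENDER, clears the targets, then runs DrawCall per mesh with its own materials.
; DrawCall projects each triangle from light and camera, drawing depth, UV and vertex normals as canvas triangles, then full-target pixel normal, base color and MSR passes.
; Copied temp targets serve as Z-buffers; a delayed loop spreads triangles over time.
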(event EventBeginPlay
  (bind _spotlight (Variables|Default|GetSpotLight))
  (bind _relativerotation (Variables|/Script/Engine.SceneComponent|GetRelativeRotation _spotlight))
  (Utilities|FlowControl|Sequence
    (:then_0
      (Rendering|Material|SetVectorParameterValue "/Game/BPrender/RenderMaterials/MPC_RENDER.MPC_RENDER" "Forward" (Math|Conversions|ToLinearColor(Vector) (Math|Vector|GetForwardVector _relativerotation)) :!class /Script/Engine.KismetMaterialLibrary)
      (Rendering|Material|SetVectorParameterValue "/Game/BPrender/RenderMaterials/MPC_RENDER.MPC_RENDER" "Right" (Math|Conversions|ToLinearColor(Vector) (Math|Vector|GetRightVector _relativerotation)) :!class /Script/Engine.KismetMaterialLibrary)
      (Rendering|Material|SetVectorParameterValue "/Game/BPrender/RenderMaterials/MPC_RENDER.MPC_RENDER" "Up" (Math|Conversions|ToLinearColor(Vector) (Math|Vector|GetUpVector _relativerotation)) :!class /Script/Engine.KismetMaterialLibrary)
      (Rendering|Material|SetVectorParameterValue "/Game/BPrender/RenderMaterials/MPC_RENDER.MPC_RENDER" "Position" (Math|Conversions|ToLinearColor(Vector) (Variables|/Script/Engine.SceneComponent|GetRelativeLocation _spotlight)) :!class /Script/Engine.KismetMaterialLibrary)
      (Variables|Default|SetTLight (Transformation|GetRelativeTransform (Variables|Default|GetSpotLight))))
    (:then_1
      (Rendering|ClearRenderTarget2D "/Game/BPrender/RTs/RT_Depth.RT_Depth")
      (Rendering|ClearRenderTarget2D "/Game/BPrender/RTs/RT_UV.RT_UV")
      (Rendering|ClearRenderTarget2D "/Game/BPrender/RTs/RT_BaseColor.RT_BaseColor")
      (Rendering|ClearRenderTarget2D "/Game/BPrender/RTs/RT_MSR.RT_MSR")
      (Rendering|ClearRenderTarget2D "/Game/BPrender/RTs/RT_VN.RT_VN")
      (Rendering|ClearRenderTarget2D "/Game/BPrender/RTs/RT_PN.RT_PN")
      (Rendering|ClearRenderTarget2D "/Game/BPrender/RTs/RT_ShadowMap.RT_ShadowMap"))
    (:then_2
      (Utilities|DrawCall (Variables|Default|GetCube1) "/Game/BPrender/Demo/Tree/T_Bush_D.T_Bush_D" "/Game/BPrender/Demo/Tree/M_DrawPN_Tree.M_DrawPN_Tree" "/Game/BPrender/Demo/Tree/M_DrawBaseColor_Tree.M_DrawBaseColor_Tree" "/Game/BPrender/Demo/Tree/M_DrawMSR_Tree.M_DrawMSR_Tree")
      (Rendering|ClearRenderTarget2D "/Game/BPrender/RTs/RT_UV.RT_UV")
      (Utilities|DrawCall (Variables|Default|GetCube) "/Engine/EngineResources/WhiteSquareTexture.WhiteSquareTexture" "/Game/BPrender/Demo/Chair/M_DrawPN.M_DrawPN" "/Game/BPrender/Demo/Chair/M_DrawBaseColor.M_DrawBaseColor" "/Game/BPrender/Demo/Chair/M_DrawMSR.M_DrawMSR"))))

(fn ConstructionScript
  (bind _spotlight (Variables|Default|GetSpotLight))
  (bind _relativerotation (Variables|/Script/Engine.SceneComponent|GetRelativeRotation _spotlight))
  (Class|KismetProceduralMeshLibrary|CopyProceduralMeshfromStaticMeshComponent (Variables|Default|GetCube) 0 (Variables|Default|GetProceduralMesh) false)
  (Rendering|Material|SetVectorParameterValue "/Game/BPrender/RenderMaterials/MPC_RENDER.MPC_RENDER" "Forward" (Math|Conversions|ToLinearColor(Vector) (Math|Vector|GetForwardVector _relativerotation)) :!class /Script/Engine.KismetMaterialLibrary)
  (Rendering|Material|SetVectorParameterValue "/Game/BPrender/RenderMaterials/MPC_RENDER.MPC_RENDER" "Right" (Math|Conversions|ToLinearColor(Vector) (Math|Vector|GetRightVector _relativerotation)) :!class /Script/Engine.KismetMaterialLibrary)
  (Rendering|Material|SetVectorParameterValue "/Game/BPrender/RenderMaterials/MPC_RENDER.MPC_RENDER" "Up" (Math|Conversions|ToLinearColor(Vector) (Math|Vector|GetUpVector _relativerotation)) :!class /Script/Engine.KismetMaterialLibrary)
  (Rendering|Material|SetVectorParameterValue "/Game/BPrender/RenderMaterials/MPC_RENDER.MPC_RENDER" "Position" (Math|Conversions|ToLinearColor(Vector) (Variables|/Script/Engine.SceneComponent|GetRelativeLocation _spotlight)) :!class /Script/Engine.KismetMaterialLibrary))

(fn WorldtoScreen
  (params (Location :type Vector) (TCamera :type Transform%20%28by%20ref%29) (FOV :type Float%20%28double-precision%29))
  (bind _returnvalue (Math|Transform|InverseTransformLocation TCamera Location))
  (bind _returnvalue_2 (/ FOV 2.0))
  (bind _size (Variables|Default|GetSize))
  (bind (_x _y _z) (Math|Vector|BreakVector _returnvalue))
  (bind _returnvalue_3 (Math|Trig|Tan(Degrees) _returnvalue_2))
  (return (+ (* (/ (Math|Vector2D|MakeVector2D _y _z) (* (Math|Vector2D|MakeVector2D _x _x) (* (Math|Vector2D|MakeVector2D 1.0 (/ (.y _size) (.x _size))) (Math|Vector2D|MakeVector2D _returnvalue_3 _returnvalue_3)))) "(X=0.500000,Y=-0.500000)") "(X=0.500000,Y=0.500000)") _x))

(fn ToDepthParam
  (params (Position :type Vector%202D%20Structure) (MeshUV :type Vector%202D%20Structure))
  (bind (_x _y) (Math|Vector2D|BreakVector2D MeshUV))
  (bind (_x_2 _y_2) (Math|Vector2D|BreakVector2D Position))
  (return (Utilities|Struct|MakeLinearColor _x_2 _y_2 _x _y)))

(fn DepthHelper
  (params (TCamera :type Transform) (TMesh :type Transform) (UVa :type Vector%202D%20Structure) (UVb :type Vector%202D%20Structure) (UVc :type Vector%202D%20Structure) (Size :type Vector%202D%20Structure) (Pa :type Vector) (Pb :type Vector) (Pc :type Vector) (FOV :type Float%20%28double-precision%29))
  (bind _returnvalue (Math|Transform|TransformLocation TMesh Pa))
  (bind _returnvalue_2 (Math|Transform|TransformLocation TMesh Pc))
  (bind _returnvalue_3 (Math|Transform|TransformLocation TMesh Pb))
  (bind (_returnvalue_4 _z) (CallFunction|WorldtoScreen _returnvalue_2 TCamera FOV))
  (bind (_returnvalue_5 _z_2) (CallFunction|WorldtoScreen _returnvalue TCamera FOV))
  (bind (_returnvalue_6 _z_3) (CallFunction|WorldtoScreen _returnvalue_3 TCamera FOV))
  (return (Utilities|Array|MakeArray (Utilities|Struct|MakeCanvasUVTri (* Size _returnvalue_5) _returnvalue_5 "(R=1.000000,G=1.000000,B=1.000000,A=1.000000)" (* Size _returnvalue_6) _returnvalue_6 "(R=1.000000,G=1.000000,B=1.000000,A=1.000000)" (* Size _returnvalue_4) _returnvalue_4 "(R=1.000000,G=1.000000,B=1.000000,A=1.000000)")) (CallFunction|ToDepthParam _returnvalue_5 UVa) (CallFunction|ToDepthParam _returnvalue_6 UVb) (CallFunction|ToDepthParam _returnvalue_4 UVc) (Math|Color|MakeColor (/ 1.0 _z_2) (/ 1.0 _z_3) (/ 1.0 _z))))